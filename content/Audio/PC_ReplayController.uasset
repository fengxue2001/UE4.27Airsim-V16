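; Player controller for replay playback, with spectating and pause control.
; On begin play it prints its name, then, if local and playing a replay, shows the cursor, sets Game and UI input and spectates the ThirdPersonView of the first BP_FlyingPawn found.
; The space bar toggles replay pause and resume.
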(event `self.ReceiveBeginPlay`
  (`KismetSystemLibrary.PrintString` (`KismetSystemLibrary.GetDisplayName` self) true true (struct :`G` 0.66 :`B` 1.0 :`A` 1.0) 20.0)
  (if (`self.IsLocalController`)
    (if (`ReplaySystemBPLibrary.IsPlayingReplay`)
      (set `self.bShowMouseCursor` true)
      (`WidgetBlueprintLibrary.SetInputMode_GameAndUIEx` self null "DoNotLock" false)
      (bind _outactors (`GameplayStatics.GetAllActorsOfClass` "/AirSim/Blueprints/BP_FlyingPawn.BP_FlyingPawn_C"))
      (`ReplaySystemBPLibrary.SpectateActor` (`/AirSim/Blueprints/BP_FlyingPawn.ThirdPersonView` (`|GetArrayItem` _outactors))))))

(event `Key|SpaceBar`
  (params (Key :type "Key Structure"))
  ;[1 1 1] 点击空格进行暂停
  (:`Pressed`
    (if (`ReplaySystemBPLibrary.IsReplayPlaybackPaused`)
      (`ReplaySystemBPLibrary.ResumePlayback`)
      (else
        (`ReplaySystemBPLibrary.PausePlayback`)))))

(fn `UserConstructionScript`)